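; Player character "lilfella" with side-scroller style controls: horizontal movement and jumping.
; The horizontal axis adds movement along world Y and mirrors the Playerrun component by flipping its X scale to match direction.
; Space calls Jump, while the vertical axis, BeginPlay and Tick are empty.
; An unfinished line-trace ground check with debug prints and a world-X movement call are disconnected and never run.
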(event `self.ReceiveBeginPlay`)

(event `InputAxis|vertical`
  (params (AxisValue :type "Float (single-precision)")))

(event `InputAxis|horizontal`
  (params (AxisValue :type "Float (single-precision)"))
  (bind _playerrun (`self.playerrun`))
  (`self.AddMovementInput` (0.0 1.0 0.0) AxisValue)
  (if (> AxisValue 0.0)
    (`SceneComponent.SetRelativeScale3D` _playerrun (5.0 5.0 5.0))
    (elif (< AxisValue 0.0)
      (`SceneComponent.SetRelativeScale3D` _playerrun (-5.0 5.0 5.0)))))

(event `Key|SpaceBar`
  (params (Key :type "Key Structure"))
  (:`Pressed`
    (`self.Jump`)))

(event `self.ReceiveTick`
  (params (DeltaSeconds :type "Float (single-precision)")))

(fn `UserConstructionScript`)